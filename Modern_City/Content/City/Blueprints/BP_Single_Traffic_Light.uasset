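; Pedestrian traffic light prop for the city that colors itself at construction time and has no active runtime logic.
; The construction script picks a vector color from a Material Parameter Collection, either by a clamped index or randomly using a stream seeded from actor location.
; It writes that color into default Custom Primitive Data on the traffic light component and its direct primitive children.
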(event EventBeginPlay)

(event Collision|EventActorBeginOverlap
  (params (OtherActor :type Actor%20Object%20Reference)))

(event EventTick
  (params (DeltaSeconds :type Float%20%28single-precision%29)))

(fn ConstructionScript
  (bind _returnvalue (Transformation|GetActorLocation))
  (bind _mpc (Variables|Components|GetMPC))
  (bind _returnvalue_2 (Class|MaterialParameterCollection|GetVectorParameterNames _mpc))
  (bind (_x _y _z) (Math|Vector|BreakVector _returnvalue))
  (bind _returnvalue_3 (Utilities|Array|Length _returnvalue_2))
  (bind _returnvalue_4 (- _returnvalue_3 1))
  ;[1 1 1] Random Seed based on Position
  (Math|Random|SetRandomStreamSeed (Variables|Components|GetRandom%20Stream) (Math|Float|Truncate (+ _x _y _z)))
  (bind _returnvalue_5 (Rendering|Material|GetVectorParameterValue (Variables|Components|GetMPC) (Utilities|Array|Get(acopy) _returnvalue_2 (Math|Integer|SelectInt (Math|Random|RandomIntegerinRangefromStream (Variables|Components|GetRandom%20Stream) 0 _returnvalue_4) (Math|Integer|Clamp(Integer) (Variables|Components|GetArrayColor) 0 _returnvalue_4) (Variables|Components|GetRandomColors?))) :!class /Script/Engine.KismetMaterialLibrary))
  (for _array_element (Components|GetChildrenComponents (Variables|Default|GetMM00277_Traffic_Light_Pedestrian) false)
    (bind _asprimitive_component (Utilities|Casting|CastToPrimitiveComponent _array_element))
    ;[1 1 1] Set Color
    (Rendering|Material|SetDefaultCustomPrimitiveDataVector4 _asprimitive_component 0 (Math|Vector4|MakeVector4 (.R (Math|Color|BreakColor _returnvalue_5)) (.G (Math|Color|BreakColor _returnvalue_5)) (.B (Math|Color|BreakColor _returnvalue_5)) 1.0))))