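; Wind controller actor for Maxtree foliage presets that sets global wind parameters from its placement and exposed variables.
; Its construction script writes the actor's forward vector as wind direction into the MP_MT_PM_Wind_Control material parameter collection, alongside scalar wind and wave settings.
; All work happens at construction time; the BeginPlay, overlap and Tick events are empty, so nothing updates during play.
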(event EventBeginPlay)

(event Collision|EventActorBeginOverlap
  (params (OtherActor :type Actor%20Object%20Reference)))

(event EventTick
  (params (DeltaSeconds :type Float%20%28single-precision%29)))

(fn ConstructionScript
  (Rendering|Material|SetVectorParameterValue "/Maxtree/Maxtree/MaxtreePresets/MPCs/MP_MT_PM_Wind_Control.MP_MT_PM_Wind_Control" "Global_Wind_Direction" (Math|Conversions|ToLinearColor(Vector) (Transformation|GetActorForwardVector)) :!class /Script/Engine.KismetMaterialLibrary)
  (Rendering|Material|SetScalarParameterValue "/Maxtree/Maxtree/MaxtreePresets/MPCs/MP_MT_PM_Wind_Control.MP_MT_PM_Wind_Control" "Global_Wind_Speed" (Variables|Wind|GetGlobal_Wind_Speed) :!class /Script/Engine.KismetMaterialLibrary)
  (Rendering|Material|SetScalarParameterValue "/Maxtree/Maxtree/MaxtreePresets/MPCs/MP_MT_PM_Wind_Control.MP_MT_PM_Wind_Control" "Global_Wind_Intensity" (Variables|Wind|GetGlobal_Wind_Intensity) :!class /Script/Engine.KismetMaterialLibrary)
  (Rendering|Material|SetScalarParameterValue "/Maxtree/Maxtree/MaxtreePresets/MPCs/MP_MT_PM_Wind_Control.MP_MT_PM_Wind_Control" "Global_Wave_Scale" (Variables|Wind|GetGlobal_Wave_Scale) :!class /Script/Engine.KismetMaterialLibrary)
  (Rendering|Material|SetScalarParameterValue "/Maxtree/Maxtree/MaxtreePresets/MPCs/MP_MT_PM_Wind_Control.MP_MT_PM_Wind_Control" "Global_Wave_Speed" (Variables|Wind|GetGlobal_Wave_Speed) :!class /Script/Engine.KismetMaterialLibrary)
  (Rendering|Material|SetScalarParameterValue "/Maxtree/Maxtree/MaxtreePresets/MPCs/MP_MT_PM_Wind_Control.MP_MT_PM_Wind_Control" "Global_Wave_Max_Bend_Angle" (Variables|Wind|GetGlobal_Wave_Max_Bend_Angle) :!class /Script/Engine.KismetMaterialLibrary)
  (Rendering|Material|SetScalarParameterValue "/Maxtree/Maxtree/MaxtreePresets/MPCs/MP_MT_PM_Wind_Control.MP_MT_PM_Wind_Control" "Global_Wave_Disturbance" (Variables|Wind|GetGlobal_Wave_Disturbance) :!class /Script/Engine.KismetMaterialLibrary))