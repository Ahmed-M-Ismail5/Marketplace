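; Boat bobbing Blueprint that continuously moves and tilts its actor to fake floating on water.
; On BeginPlay it saves the location and starts two looping timelines at configurable play rates, with random values passed to Play, apparently to vary phase.
; One timeline offsets the saved location, while the other sets rotation absolutely from a maximum rotation, ignoring the starting rotation.
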(event EventBeginPlay
  (Components|Timeline|SetPlayRate (Variables|Default|GetTimeline) (Variables|Default|GetOffsetPlayRate))
  (Components|Timeline|SetPlayRate (Variables|Default|GetTimeline_0) (Variables|Default|GetRotationPlayRate))
  (Variables|Default|SetSavedLocation (Transformation|GetActorLocation))
  (Utilities|FlowControl|Sequence
    (:then_0
      (bind _newtrack_0 (Timeline|Timeline Play)
        (:Update
          (Transformation|SetActorLocation (+ (Variables|Default|GetSavedLocation) (* _newtrack_0 (Variables|Default|GetDisplacementOffsetMax))) false true))
        (:Finished
          (Timeline|Timeline PlayFromStart))))
    (:then_1
      (bind _newtrack_0_2 (Timeline|Timeline_0 Play)
        (:Update
          (Transformation|SetActorRotation (* (Variables|Default|GetRotationOffsetMax) _newtrack_0_2) true))
        (:Finished
          (Timeline|Timeline_0 PlayFromStart))))))

(event Collision|EventActorBeginOverlap
  (params (OtherActor :type Actor%20Object%20Reference)))

(event EventTick
  (params (DeltaSeconds :type Float%20%28single-precision%29))
  (CallFunction|TimelineUpdateFunc))

(fn ConstructionScript)