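; Actor that temporarily overrides Lumen global illumination and reflection quality settings on every PostProcessVolume in the level.
; Custom events call enable and disable functions, guarded by an IsOverriden flag, that write the configured methods and quality values or restore saved settings.
; An optional reset step precedes the override.
; A single variable stores original settings, so disabling applies the last saved volume's settings to all volumes.
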(event Custom|CE_EnableOverridingQualitySettings
  (CallFunction|EnableQualityOverrides))

(event Custom|CE_DisableOverridingQualitySettings
  (CallFunction|DisableQualityOverrides))

(event EventBeginPlay)

(event Collision|EventActorBeginOverlap
  (params (OtherActor :type Actor%20Object%20Reference)))

(event EventTick
  (params (DeltaSeconds :type Float%20%28single-precision%29)))

(fn ConstructionScript)

(fn EnableQualityOverrides
  (if (Variables|Default|GetIsOverriden?)
    (Development|PrintString "Post Processing is already overriden.")
    (else
      (bind _outactors (Actor|GetAllActorsOfClass "/Script/Engine.PostProcessVolume"))
      (for _array_element _outactors
        (Utilities|IsValid _array_element
          (:Is%20Valid
            (bind _output_get (Variables|Default|SetPostProcessSettings_SceneOriginal (Variables|/Script/Engine.PostProcessVolume|GetSettings _array_element)))
            ;[1 0.3646 0.3646] Whether to Reset the Settings to Engine Default values or use a Custom Settings defined in the map.
            (if (Variables|Default|GetResetQualityOverridingsToDefault)
              (bind _structout (Utilities|Struct|SetmembersinPostProcessSettings _output_get "Lumen"))
              (bind _structout_2 (Utilities|Struct|SetmembersinPostProcessSettings _structout "Lumen"))
              (Variables|Default|SetPostProcessSettings_SceneOriginal _structout_2))
            (bind _output_get_2 (Variables|Default|SetPostProcessSettings_SceneOverride (Variables|Default|GetPostProcessSettings_SceneOriginal)))
            (bind _structout_3 (Utilities|Struct|SetmembersinPostProcessSettings _output_get_2 (Variables|LumenGlobalIllumination|GetMethod%20GI) (Variables|LumenReflections|GetRay%20Lighting%20Mode) (Variables|LumenGlobalIllumination|GetLumen%20Scene%20Lighting%20Quality) (Variables|LumenGlobalIllumination|GetLumen%20Scene%20Detail) (Variables|LumenGlobalIllumination|GetFinal%20Gather%20Quality) (Variables|LumenGlobalIllumination|GetScene%20Capture%20Cache%20Resolution%20Scale) (Variables|LumenReflections|GetMethod%20Reflections) (Variables|LumenReflections|GetQuality)))
            (Variables|/Script/Engine.PostProcessVolume|SetSettings _array_element _structout_3)
            (Variables|Default|SetIsOverriden? true)))))))

(fn DisableQualityOverrides
  (if (Variables|Default|GetIsOverriden?)
    (bind _outactors (Actor|GetAllActorsOfClass "/Script/Engine.PostProcessVolume"))
    (for _array_element _outactors
      (Utilities|IsValid _array_element
        (:Is%20Valid
          (Variables|/Script/Engine.PostProcessVolume|SetSettings _array_element (Variables|Default|GetPostProcessSettings_SceneOriginal))
          (Variables|Default|SetIsOverriden? false))))
    (else
      (Development|PrintString "Post Processing has not been overriden yet."))))