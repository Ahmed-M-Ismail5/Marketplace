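; BP_Weathering generates rain drip textures for weathering effects by redrawing render targets every frame.
; BeginPlay creates three dynamic materials sharing resolution and drip scale settings, with later passes sampling the preceding pass's render target.
; Tick runs the chain: mask generation, blur, then final output into the third target.
; The first target resets to a half-red, half-green color each tick and at EndPlay.
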(event EventBeginPlay
  (bind _rt_drips_1 (Variables|Default|GetRT_Drips_1))
  (bind _drips_scale (Variables|Default|GetDrips_Scale))
  (bind _returnvalue (Math|Conversions|ToFloat(Integer) _drips_scale))
  (bind _sizex (Variables|/Script/Engine.TextureRenderTarget2D|GetSizeX _rt_drips_1))
  (bind _sizey (Variables|/Script/Engine.TextureRenderTarget2D|GetSizeY _rt_drips_1))
  (bind _returnvalue_2 (Math|Conversions|ToFloat(Integer) _sizex))
  (bind _returnvalue_3 (Math|Conversions|ToFloat(Integer) _sizey))
  (bind _returnvalue_4 (Math|Vector|MakeVector _returnvalue_2 _returnvalue_3 _returnvalue))
  (bind _returnvalue_5 (Math|Conversions|ToLinearColor(Vector) _returnvalue_4))
  (Utilities|FlowControl|Sequence
    (:then_0
      (bind _returnvalue_6 (Rendering|Material|CreateDynamicMaterialInstance (Variables|Default|GetM_Drips_1) "DMI_Drips_1" "None" :!class /Script/Engine.KismetMaterialLibrary))
      (Variables|Default|SetDMI_Drips_1 _returnvalue_6)
      (Rendering|Material|SetVectorParameterValue (Variables|Default|GetDMI_Drips_1) "Settings" _returnvalue_5 :!class /Script/Engine.MaterialInstanceDynamic))
    (:then_1
      (bind _returnvalue_7 (Rendering|Material|CreateDynamicMaterialInstance (Variables|Default|GetM_Drips_2) "DMI_Drips_2" "None" :!class /Script/Engine.KismetMaterialLibrary))
      (bind _output_get (Variables|Default|SetDMI_Drips_2 _returnvalue_7))
      (Rendering|Material|SetTextureParameterValue _output_get "Tex" (Variables|Default|GetRT_Drips_1))
      (Rendering|Material|SetVectorParameterValue (Variables|Default|GetDMI_Drips_2) "Settings" _returnvalue_5 :!class /Script/Engine.MaterialInstanceDynamic))
    (:then_2
      (bind _returnvalue_8 (Rendering|Material|CreateDynamicMaterialInstance (Variables|Default|GetM_Drips_3) "DMI_Drips_3" "None" :!class /Script/Engine.KismetMaterialLibrary))
      (bind _output_get_2 (Variables|Default|SetDMI_Drips_3 _returnvalue_8))
      (Rendering|Material|SetTextureParameterValue _output_get_2 "Tex" (Variables|Default|GetRT_Drips_2))
      (Rendering|Material|SetVectorParameterValue (Variables|Default|GetDMI_Drips_3) "Settings" _returnvalue_5 :!class /Script/Engine.MaterialInstanceDynamic))))

(event EventEndPlay
  (params (EndPlayReason :type EEndPlayReason%20Enum :default "Destroyed"))
  (Rendering|ClearRenderTarget2D (Variables|Default|GetRT_Drips_1) "(R=0.500000,G=0.500000,B=0.000000,A=1.000000)"))

(event EventTick
  (params (DeltaSeconds :type Float%20%28single-precision%29))
  (Rendering|ClearRenderTarget2D (Variables|Default|GetRT_Drips_1) "(R=0.500000,G=0.500000,B=0.000000,A=1.000000)")
  (Rendering|DrawMaterialtoRenderTarget (Variables|Default|GetRT_Drips_1) (Variables|Default|GetDMI_Drips_1)) ; 1 : Generate Masks
  (Rendering|DrawMaterialtoRenderTarget (Variables|Default|GetRT_Drips_2) (Variables|Default|GetDMI_Drips_2)) ; 2 : Blur
  (Rendering|DrawMaterialtoRenderTarget (Variables|Default|GetRT_Drips_3) (Variables|Default|GetDMI_Drips_3)) ; 3 : Final Output
)

(fn ConstructionScript)