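; Traffic generator that fills a spline with weighted random vehicles for short driving sequences.
; Seeded density rolls place jittered vehicles in evenly spaced slots, as child-actor previews in construction.
; On BeginPlay it snaps spline points to the road by trace, then respawns vehicles as real actors (for Take Recorder) with FollowSpline components driving them.
; Kill boxes at both spline ends destroy overlapping vehicles to prevent U-turns.
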(event OnComponentBeginOverlap(KillBox_Start)
  (params (OverlappedComponent :type Primitive%20Component%20Object%20Reference) (OtherActor :type Actor%20Object%20Reference) (OtherComp :type Primitive%20Component%20Object%20Reference) (OtherBodyIndex :type Integer) (bFromSweep :type Boolean) (SweepResult :type Hit%20Result%20Structure%20%28by%20ref%29))
  (bind _returnvalue (Actor|GetComponentbyClass OtherActor "/Hillside/Hillside/Blueprints/FollowSplineComponent.FollowSplineComponent_C"))
  ;[1 1 1] Get rid of any vehicles at the end of the spline to prevent U-turns. We're only simulating a short sequence, so no need to make perfect loops
  (if (Utilities|IsValid _returnvalue)
    (Components|DestroyComponent _returnvalue) ; FollowSpline component gets left \nbehind for some reason when \nkilling child actor component
    (Utilities|FlowControl|Delay 0.1) ; FollowSpline component seems to take \none extra frame to die. Adding delay to avoid \nmissing references to parent actor we're \nabout to kill
    (if (Utilities|IsValid OtherActor) ; Avoiding some occasional \ngarbage collection errors
      (Actor|DestroyActor OtherActor))))

(event OnComponentBeginOverlap(KillBox_End)
  (params (OverlappedComponent :type Primitive%20Component%20Object%20Reference) (OtherActor :type Actor%20Object%20Reference) (OtherComp :type Primitive%20Component%20Object%20Reference) (OtherBodyIndex :type Integer) (bFromSweep :type Boolean) (SweepResult :type Hit%20Result%20Structure%20%28by%20ref%29))
  (bind _returnvalue (Actor|GetComponentbyClass OtherActor "/Hillside/Hillside/Blueprints/FollowSplineComponent.FollowSplineComponent_C"))
  ;[1 1 1] Get rid of any vehicles at the end of the spline to prevent U-turns. We're only simulating a short sequence, so no need to make perfect loops
  (if (Utilities|IsValid _returnvalue)
    (Components|DestroyComponent _returnvalue)
    (Utilities|FlowControl|Delay 0.1)
    (if (Utilities|IsValid OtherActor)
      (Actor|DestroyActor OtherActor))))

(event Custom|PopulateVehicles
  (params (InPlay :type Boolean))
  (bind _childactors (Actor|GetAllChildActors true))
  (bind _vehiclespacing (Variables|Default|GetVehicleSpacing))
  (bind _vehiclegrabbag (Variables|Default|GetVehicleGrabBag))
  (bind _stream (Variables|Default|GetStream))
  (bind _vehiclelist (Variables|Default|GetVehicleList))
  (bind _spline (Variables|Default|GetSpline))
  (bind _returnvalue (* _vehiclespacing 0.15))
  (Variables|Default|SetIsInGame InPlay)
  (while (> (Utilities|Array|Length _childactors) 0)
    (Actor|DestroyActor _childactors) ; When in Play, first get rid of temporary \nChild Actors from Construction Script.
  )
  (Utilities|Array|Clear (Variables|Default|GetVehicleGrabBag))
  ;[1 1 1] Use existing stream (random seed), or make new one
  (Class|KismetMathLibrary|ResetRandomStream _stream)
  (if (Variables|Default|GetGenerateNewSeed)
    (Class|KismetMathLibrary|SeedRandomStream _stream))
  (if (Utilities|IsValid (Game|GetGameMode)) ; Can't delay in construction script
    (Utilities|FlowControl|Delay 0.0) ; In extremely heavy levels, SpawnActorFromClass \ncannot finish adding actors when called from \nthe construction script. Giving the level one frame \nof warm-up before trying avoids errors in this \nparticular case.
  )
  (Utilities|FlowControl|Sequence
    (:then_0
      ;[1 1 1] Create a grab bag of selected vehicles based on their given weighting
      (bind _keys (Utilities|Map|Keys _vehiclelist))
      (for _array_element _keys ; For every vehicle in the list.....
        (for _index (range 0 (- (.Value (Utilities|Map|Find _vehiclelist _array_element)) 1)) ; ... and add that number of class copies to our grab bag
          (Utilities|Array|Add (Variables|Default|GetVehicleGrabBag) _array_element))))
    (:then_1
      ;[1 1 1] For every possible vehicle slot, roll the dice with our density multiplier to see if something should be there.
      (for _index_2 (range 0 (- (Math|Float|Truncate (/ (Spline|GetSplineLength (Variables|Default|GetSpline)) (Variables|Default|GetVehicleSpacing))) 1))
        (bind _output_get (Variables|Default|SetRandomSpawnChance (Class|KismetMathLibrary|RandomBoolwithWeightfromStream (Variables|Default|GetStream) (Variables|Default|GetDensity))))
        (if _output_get
          (Variables|Default|SetRandomJitter (Math|Random|RandomFloatinRangefromStream (Variables|Default|GetStream) (* _returnvalue 1.0) (* _returnvalue -1.0)))
          (Variables|Default|SetSavedVehicleIndex (Math|Random|RandomIntegerinRangefromStream (Variables|Default|GetStream) 0 (- (Utilities|Array|Length _vehiclegrabbag) 1)))
          (if (Variables|Default|GetIsInGame) ; We need real actors for the Take Recorder, \nbut only child actors can be created \non Construction script
            ;[1 1 1] Spawn "real" actors when playing and simulating
            (bind _returnvalue_2 (Game|SpawnActorfromClass (Utilities|Array|Get(acopy) _vehiclegrabbag (Variables|Default|GetSavedVehicleIndex)) (Math|Transform|MakeTransform (Spline|GetLocationatDistanceAlongSpline _spline (+ (* _index_2 (Variables|Default|GetVehicleSpacing)) (Variables|Default|GetRandomJitter)) (select (Variables|Default|GetIsInGame) "World" "Local")) (Math|Rotator|MakeRotator (.roll (Spline|GetRotationatDistanceAlongSpline _spline (+ (* _index_2 (Variables|Default|GetVehicleSpacing)) (Variables|Default|GetRandomJitter)) (select (Variables|Default|GetIsInGame) "World" "Local"))) (.pitch (Spline|GetRotationatDistanceAlongSpline _spline (+ (* _index_2 (Variables|Default|GetVehicleSpacing)) (Variables|Default|GetRandomJitter)) (select (Variables|Default|GetIsInGame) "World" "Local"))) (+ (.yaw (Spline|GetRotationatDistanceAlongSpline _spline (+ (* _index_2 (Variables|Default|GetVehicleSpacing)) (Variables|Default|GetRandomJitter)) (select (Variables|Default|GetIsInGame) "World" "Local"))) (* (Math|Conversions|ToFloat(Boolean) (Variables|Default|GetReverseDirection)) 1.8e+02))) "1.000000,1.000000,1.000000") "Undefined" "SelectDefaultAtRuntime" 0 0))
            (Transformation|AttachActorToActor _returnvalue_2 self "None" "KeepWorld" "KeepWorld" "KeepWorld" true)
            ;[1 1 1] Add the FollowSpline component and assign proper values from this Blueprint
            (bind _returnvalue_3 (AddComponent|AddFollowSplineComponent _returnvalue_2))
            (Variables|/Hillside/Hillside/Blueprints/FollowSplineComponent.FollowSplineComponent_C|SetTargetSplineComponent _returnvalue_3 (Variables|Default|GetSpline))
            (Components|Activation|Activate _returnvalue_3 false)
            (Variables|/Hillside/Hillside/Blueprints/FollowSplineComponent.FollowSplineComponent_C|SetSpeed _returnvalue_3 1.0)
            (Variables|/Hillside/Hillside/Blueprints/FollowSplineComponent.FollowSplineComponent_C|SetMaxSpeed%20cm/s _returnvalue_3 (* (Variables|Default|GetSpeed%20%28km/h%29) 27.78))
            (if (or (Utilities|String|Contains (Utilities|GetClassDisplayName (Utilities|GetClass _returnvalue_2)) "truck") (Utilities|String|Contains (Utilities|GetClassDisplayName (Utilities|GetClass _returnvalue_2)) "bus")) ; Large vehicles need a different\n ForwardAimDistance
              (Variables|/Hillside/Hillside/Blueprints/FollowSplineComponent.FollowSplineComponent_C|SetForwardAimDistance _returnvalue_3 1.2e+03)
              (else
                (Variables|/Hillside/Hillside/Blueprints/FollowSplineComponent.FollowSplineComponent_C|SetForwardAimDistance _returnvalue_3 7e+02)))
            (else
              ;[1 1 1] Spawn Child Actors for preview in editor
              (bind _returnvalue_4 (AddComponent|AddChildActorComponent false (Math|Transform|MakeTransform (Spline|GetLocationatDistanceAlongSpline _spline (+ (* _index_2 (Variables|Default|GetVehicleSpacing)) (Variables|Default|GetRandomJitter)) (select (Variables|Default|GetIsInGame) "World" "Local")) (Math|Rotator|MakeRotator (.roll (Spline|GetRotationatDistanceAlongSpline _spline (+ (* _index_2 (Variables|Default|GetVehicleSpacing)) (Variables|Default|GetRandomJitter)) (select (Variables|Default|GetIsInGame) "World" "Local"))) (.pitch (Spline|GetRotationatDistanceAlongSpline _spline (+ (* _index_2 (Variables|Default|GetVehicleSpacing)) (Variables|Default|GetRandomJitter)) (select (Variables|Default|GetIsInGame) "World" "Local"))) (+ (.yaw (Spline|GetRotationatDistanceAlongSpline _spline (+ (* _index_2 (Variables|Default|GetVehicleSpacing)) (Variables|Default|GetRandomJitter)) (select (Variables|Default|GetIsInGame) "World" "Local"))) (* (Math|Conversions|ToFloat(Boolean) (Variables|Default|GetReverseDirection)) 1.8e+02))) "1.000000,1.000000,1.000000")))
              (ChildActorComponent|SetChildActorClass _returnvalue_4 (Utilities|Array|Get(acopy) _vehiclegrabbag (Variables|Default|GetSavedVehicleIndex)))))))
      (Variables|Default|SetGenerateNewSeed false) ; Always reset our randomization button
    )))

(event EventBeginPlay
  (bind _spline (Variables|Default|GetSpline))
  (Class|SplineComponent|SetDrawDebug _spline true)
  ;[1 1 1] Align spline control points to road surface - always checks below the point, so point must be above road
  (for _index (range 0 (- (Spline|GetNumberOfSplinePoints _spline) 1))
    (bind _outhit (Collision|LineTraceByChannel (+ (Spline|GetLocationatSplinePoint (Variables|Default|GetSpline) _index "World") "0.000000,0.000000,150.000000") (- (Spline|GetLocationatSplinePoint (Variables|Default|GetSpline) _index "World") "0.000000,0.000000,10000.000000") "TraceTypeQuery1" true 0 "None"))
    (Spline|SetLocationatSplinePoint (Variables|Default|GetSpline) _index (.location _outhit) "World" true))
  ;[0.5301 1 0.4921] Create vehicles that drive
  (CallFunction|PopulateVehicles true))

(fn ConstructionScript
  (bind _spline (Variables|Default|GetSpline))
  (CallFunction|PopulateVehicles false)
  ;[1 1 1] Create Kill Boxes for traffic that reach the end of a spline
  (bind _returnvalue (AddComponent|AddBoxComponent false (Math|Transform|MakeTransform (Spline|GetLocationatSplinePoint _spline 0 "Local") "0, 0, 0" "1.000000,1.000000,1.000000")))
  (Variables|Default|SetKillBox_Start _returnvalue)
  (bind _returnvalue_2 (AddComponent|AddBoxComponent false (Math|Transform|MakeTransform (Spline|GetLocationatSplinePoint _spline (- (Spline|GetNumberOfSplinePoints _spline) 1) "Local") "0, 0, 0" "1.000000,1.000000,1.000000")))
  (Variables|Default|SetKillBox_End _returnvalue_2))